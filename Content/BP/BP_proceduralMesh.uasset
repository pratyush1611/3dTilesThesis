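; Actor Blueprint that experiments with building a small cube procedurally from eight hard-coded corner vertices.
; The Construction Script appends further triangle index lists to an inline two-triangle array, then creates a ProceduralMesh section with CreateMeshSectionLinearColor.
; The indices live in an array literal rather than a variable, and the section call shows only the base two triangles.
; No normals, UVs or colors are supplied, and the event graph is inactive.
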(event EventBeginPlay)

(event Collision|EventActorBeginOverlap
  (params (OtherActor :type Actor%20Object%20Reference)))

(event EventTick
  (params (DeltaSeconds :type Float%20%28single-precision%29)))

(fn ConstructionScript
  (bind _array (Utilities|Array|MakeArray 2 1 0 3 1 2))
  (Utilities|Array|AppendArray _array (Utilities|Array|MakeArray 2 0 6 6 0 1))
  (Utilities|Array|AppendArray _array (Utilities|Array|MakeArray 2 6 7 7 3 2))
  (Utilities|Array|AppendArray _array (Utilities|Array|MakeArray 4 0 5 5 0 1))
  (Utilities|Array|AppendArray _array (Utilities|Array|MakeArray 1 5 6 6 5 7))
  (Utilities|Array|AppendArray _array (Utilities|Array|MakeArray 3 7 1 1 7 5))
  (Class|ProceduralMeshComponent|CreateMeshSectionLinearColor (Variables|Default|GetProceduralMesh) 0 (Utilities|Array|MakeArray "0.000000,0.000000, 0" "0,10.000000,0.000000" "10.000000,0.000000,0.000000" "10.000000,10.000000,0.000000" "0.000000, 0,10.000000" "0.000000,10.000000,10.000000" "10.000000,0.000000,10.000000" "10.000000,10.000000,10.000000") _array 0 0 0 0 0 0 0 false))