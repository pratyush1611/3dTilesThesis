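; BP_Gizmo_axis is an in-world transform gizmo that moves and rotates a picked component with the mouse.
; N toggles the gizmo, attaching the component under the cursor to its Rotation component, then detaching it and hiding the gizmo.
; Left-click traces for a handle; Tick projects the cursor ray offset onto that axis to move GizmoRoot, or turns mouse X into yaw for the Rotation handle.
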(event EventBeginPlay
  (Input|EnableInput (Game|GetPlayerController 0)))

(event Collision|EventActorBeginOverlap
  (params (OtherActor :type Actor%20Object%20Reference)))

(event EventTick
  (params (DeltaSeconds :type Float%20%28single-precision%29))
  (bind _returnvalue (Game|GetPlayerController 0))
  (bind _axisdragged (Variables|Default|GetaxisDragged))
  (bind _draglocation (Variables|Default|GetdragLocation))
  (bind (_worldlocation _worlddirection) (Game|Player|ConvertMouseLocationToWorldSpace _returnvalue))
  (bind _returnvalue_2 (Math|Conversions|ToTransform(Vector) _draglocation))
  (bind _returnvalue_3 (Math|Vector|GetForwardVector _axisdragged))
  (bind _returnvalue_4 (* _worlddirection 2e+04))
  (bind _returnvalue_5 (+ _returnvalue_4 _worldlocation))
  (bind _returnvalue_6 (Math|Transform|InverseTransformLocation _returnvalue_2 _returnvalue_5))
  (bind _returnvalue_7 (Math|Vector|ProjectVectorontoVector _returnvalue_6 _returnvalue_3))
  (switch Utilities|FlowControl|Switch|SwitchonAxis (.axisvar (Utilities|Struct|MakeDraggedAxis 0 (CallFunction|AxisComponent (Variables|Default|GetaxisDragged))))
    (:NewEnumerator0
      ;[1 1 1] move
      (Utilities|IsValid _axisdragged :!label _label
        (:Is%20Valid
          (Transformation|AddRelativeLocation (Variables|Default|GetGizmo%20Root) (Math|Vector|MakeVector (/ (.x _returnvalue_7) 1e+04) (/ (.y _returnvalue_7) 1e+04) (/ (.z _returnvalue_7) -1e+04)) false false))))
    (:NewEnumerator1
      (goto _label))
    (:NewEnumerator2
      (goto _label))
    (:NewEnumerator3
      ;[1 1 1] rotate
      (Transformation|AddLocalRotation (Variables|Default|GetRotation) (Math|Rotator|MakeRotator 0.0 0.0 (* (.DeltaX (Class|PlayerController|GetInputMouseDelta (Game|GetPlayerController 0))) 1e+01)) false false))))

(event Input|MouseEvents|LeftMouseButton
  (params (Key :type Key%20Structure :default "None"))
  (bind _returnvalue (Game|GetPlayerController 0))
  (bind (_worldlocation _worlddirection) (Game|Player|ConvertMouseLocationToWorldSpace _returnvalue))
  ;[0.5395 0.7111 1] lineTrace
  (:Pressed
    (if true
      (bind _outhit (Collision|LineTraceByChannel _worldlocation (+ (* _worlddirection 2e+04) _worldlocation) "TraceTypeQuery1" true 0 "ForDuration" false))
      (Variables|Default|SetDistanceToGrab (.Distance (Collision|BreakHitResult _outhit)))
      (switch Utilities|FlowControl|Switch|SwitchonAxis (.axisvar (Utilities|Struct|MakeDraggedAxis 0 (CallFunction|AxisComponent (.HitComponent (Collision|BreakHitResult _outhit)))))
        (:NewEnumerator0
          _)
        (:NewEnumerator1
          _)
        (:NewEnumerator2
          _))
      (Variables|Default|SetdragLocation (Math|Transform|InverseTransformLocation (Math|Conversions|ToTransform(Vector) (Math|Conversions|ToVector(Float) (Class|GameplayStatics|GetWorldOriginLocation))) (.Location (Collision|BreakHitResult _outhit))))))
  (:Released
    (if true
      (Variables|Default|SetaxisDragged 0))))

(event Input|KeyboardEvents|N
  (params (Key :type Key%20Structure :default "None"))
  (bind _returnvalue (Game|GetPlayerController 0))
  (bind (_worldlocation _worlddirection) (Game|Player|ConvertMouseLocationToWorldSpace _returnvalue))
  (:Pressed
    (Utilities|FlowControl|FlipFlop
      (:A
        (Rendering|SetVisibility (Variables|Default|GetGizmo%20Root) true true)
        (bind _outhit (Collision|LineTraceByChannel _worldlocation (+ (* _worlddirection 2e+04) _worldlocation) "TraceTypeQuery1" true 0 "ForDuration" false))
        (Transformation|SetWorldLocation (Variables|Default|GetGizmo%20Root) (Math|Vector|MakeVector (.x (Transformation|GetWorldLocation (.HitComponent (Collision|BreakHitResult _outhit)))) (.y (Transformation|GetWorldLocation (.HitComponent (Collision|BreakHitResult _outhit)))) (+ (.z (Transformation|GetWorldLocation (.HitComponent (Collision|BreakHitResult _outhit)))) 1e+03)) false false)
        (Transformation|AttachComponentToComponent (.HitComponent (Collision|BreakHitResult _outhit)) (Variables|Default|GetRotation) "None" "KeepWorld" "KeepWorld" "KeepRelative" true))
      (:B
        (Transformation|DetachFromComponent (.HitComponent (Collision|BreakHitResult _outhit)) "KeepWorld" "KeepWorld" "KeepRelative" true)
        (Rendering|SetVisibility (Variables|Default|GetGizmo%20Root) false true)))))

(fn ConstructionScript)

(fn AxisComponent
  (params (AxisComponent :type Primitive%20Component%20Object%20Reference))
  (Variables|Default|SetaxisDragged AxisComponent)
  (if (== (Variables|Default|GetaxisDragged) (Variables|Default|GetX))
    (return "NewEnumerator0")
    (elif (== (Variables|Default|GetaxisDragged) (Variables|Default|GetY))
      (return "NewEnumerator1")
      (elif (== (Variables|Default|GetaxisDragged) (Variables|Default|GetZ))
        (return "NewEnumerator2")
        (elif (== (Variables|Default|GetaxisDragged) (Variables|Default|GetRotation))
          (return "NewEnumerator3"))))))