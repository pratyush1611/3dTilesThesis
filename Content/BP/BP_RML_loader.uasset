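; Actor Blueprint that loads a mesh, texture and normal map from files at runtime.
; Each load destroys previous components, then builds a dynamic material from RML_BaseMaterial if both textures load.
; Each mesh node becomes a procedural mesh component with one section per submesh, parented by node index to rebuild the hierarchy.
; The material goes only to slot 0, and relative transforms apply only to child nodes.
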(event Custom|AttachToThisActor_PK
  (params (ProcMeshComp :type Procedural%20Mesh%20Component%20Object%20Reference) (parentindex :type Integer) (RelativeTransform :type Transform))
  (bind _procmesh (Variables|Default|GetProcMesh))
  ;[1 1 1] attach to actor
  (Utilities|Array|Add _procmesh ProcMeshComp)
  (if (< parentindex 0)
    (Transformation|AttachComponentToComponent ProcMeshComp (Variables|Components|GetDefaultSceneRoot) "None" "KeepRelative" "KeepRelative" "KeepRelative" true)
    (else
      (Transformation|AttachComponentToComponent ProcMeshComp (Utilities|Array|Get(acopy) _procmesh parentindex) "None" "KeepRelative" "KeepRelative" "KeepRelative" true)
      (Transformation|SetRelativeTransform ProcMeshComp RelativeTransform false false))))

(event Custom|LoadTexture_PK
  (params (TextureFilePath :type String) (NormalMapFilePath :type String))
  ;[1 1 1] texture load
  (bind (_isvalid _width _height _returnvalue) (Class|MeshLoader|LoadTexture2DfromFile TextureFilePath))
  (if _isvalid
    (bind (_isvalid_2 _width_2 _height_2 _returnvalue_2) (Class|MeshLoader|LoadTexture2DfromFile NormalMapFilePath))
    (if _isvalid_2
      (bind _returnvalue_3 (Rendering|Material|CreateDynamicMaterialInstance "/RuntimeMeshLoader/Example/RuntimeMeshLoader/RML_BaseMaterial.RML_BaseMaterial" "None" "None" :!class /Script/Engine.KismetMaterialLibrary))
      (Rendering|Material|SetTextureParameterValue _returnvalue_3 "TextureParam" _returnvalue)
      (Rendering|Material|SetTextureParameterValue _returnvalue_3 "NormalParam" _returnvalue_2)
      (Variables|Default|SetMat _returnvalue_3))))

(event Custom|LoadCustomMesh_PK
  (params (MeshFilePath :type String))
  ;[1 1 1] load mesh
  (bind _returnvalue (Class|MeshLoader|LoadMeshfromFile MeshFilePath "Absolute"))
  (if (.success _returnvalue)
    (for _array_element (.nodes _returnvalue)
      (bind _returnvalue_2 (AddComponent|AddProceduralMeshComponent true))
      (CallFunction|AttachtoThisActorPK _returnvalue_2 (.nodeparentindex _array_element) (.relativetransformtransform _array_element))
      (for (_array_element_2 _array_index) (.meshes _array_element)
        (Class|ProceduralMeshComponent|CreateMeshSectionLinearColor _returnvalue_2 _array_index (.vertices _array_element_2) (.triangles _array_element_2) (.normals _array_element_2) (.uvs _array_element_2) 0 0 0 0 (.tangents _array_element_2) false)
        (Rendering|Material|SetMaterial _returnvalue_2 0 (Variables|Default|GetMat))))
    (else
      (Development|PrintString "Could not load mesh"))))

(event Custom|ClearMeshes_PK
  (bind _procmesh (Variables|Default|GetProcMesh))
  ;[1 1 1] clear mesh
  (for _array_element _procmesh
    (Components|DestroyComponent _array_element))
  (Utilities|Array|Clear _procmesh))

(event Custom|LoadMeshAndTextureData_PK
  (params (MeshFilePath :type String) (TextureFilePath :type String) (NormalFilePath :type String))
  ;[1 1 1] load data
  (CallFunction|ClearMeshesPK)
  (CallFunction|LoadTexturePK TextureFilePath NormalFilePath)
  (CallFunction|LoadCustomMeshPK MeshFilePath))

(fn ConstructionScript)